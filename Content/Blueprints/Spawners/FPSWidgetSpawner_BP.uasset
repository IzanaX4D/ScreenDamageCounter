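; FPSWidgetSpawner_BP is a spawner actor that periodically shows screen damage widgets at random points around itself.
; On Tick it accumulates time and, once SpawnRate is exceeded, resets the timer and calls ShowScreenDamage for the first player controller with the configured widget class.
; Each call uses a random point at Radius from the actor, a random damage value, a "Damage" subtitle and yellow color.
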(event `self.ReceiveTick`
  (params (DeltaSeconds :type "Float (single-precision)"))
  (bind _time (`self.Time`))
  (if (< (`self.SpawnRate`) _time)
    (set `self.Time` 0.0)
    (`ScreenDamageFunctionLibrary.ShowScreenDamage` (`GameplayStatics.GetPlayerController` 0) (`self.WidgetClass`) (+ (* (`KismetMathLibrary.RandomUnitVector`) (`self.Radius`)) (`self.K2_GetActorLocation`)) (`KismetMathLibrary.RandomFloatInRange` 0.0 1500.0) "Damage" (`KismetMathLibrary.LinearColor_Yellow`))
    (else
      (set `self.Time` (+ _time DeltaSeconds)))))

(fn `UserConstructionScript`)